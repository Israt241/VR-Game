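; Enemy character that chases the player, melees within attack range and awards score when killed.
; A repeating AI MoveTo drives the chase, while Tick halts movement to play the attack montage and resumes it on completion.
; DamagePlayer applies damage and sound but is not called within this Blueprint.
; Lethal damage disables collision, updates score, randomly flags an ammo spawn on the game mode, then destroys the actor after a delay.
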(event `self.ReceiveBeginPlay`
  ; Activate AI Movements towards Player
  (if (not (`self.Dead?`))
    (`|AIMoveTo` self (0.0 0.0 0.0) (`GameplayStatics.GetPlayerCharacter` 0) :!label _label
      (:`OnSuccess`
        _)
      (:`OnFail`
        _))
    (`KismetSystemLibrary.Delay` 0.2)
    (goto _label)))

(event `self.ReceiveTick`
  (params (DeltaSeconds :type "Float (single-precision)"))
  ; Enemy Attack Player
  (if (`self.Can Attact?`)
    (`self.Deactivate AI Movement`)
    (`|PlayMontage` (`self.Mesh`) (`self.AttackMontage`)
      (:`OnCompleted`
        (`self.Aactivate AI Movements`)))))

(event `self.ReceiveAnyDamage`
  (params (Damage :type "Float (single-precision)") (DamageType :type "DamageType Object Reference") (InstigatedBy :type "Controller Object Reference") (DamageCauser :type "Actor Object Reference"))
  ; Enemy Died
  (if (not (`self.Dead?`))
    (bind _output_get (set `self.Health` (- (`self.Health`) Damage)))
    (if (<= _output_get 0.0)
      (`self.ExplodeEnemy`))))

(fn `Aactivate AI Movements`
  ; Activate Enemy Movement
  (`ActorComponent.Activate` (`self.CharacterMovement`) false))

(fn `Can Attact?`
  (returns (ReturnValue :type Boolean))
  ; Check if enemy can attack player on not
  (return (and (not (`self.is attacking?`)) (`self.is withing attack range?`) (not (`self.Dead?`)))))

(fn `Damage Player`
  ; Damage Player by Enemy
  (if (not (`self.Dead?`))
    (`GameplayStatics.ApplyDamage` (`GameplayStatics.GetPlayerCharacter` 0) (`self.Damage`))
    (`GameplayStatics.PlaySound2D` (`self.AttackSound`) 1.0 1.0 0.0 null null)))

(fn `Deactivate AI Movement`
  (bind _charactermovement (`self.CharacterMovement`))
  ; Deactivate Enemy Movement
  (`MovementComponent.StopMovementImmediately` _charactermovement)
  (`ActorComponent.Deactivate` _charactermovement))

(fn `is attacking?`
  (returns (ReturnValue :type Boolean))
  ; Check is Enemy attack player
  (return (`AnimInstance.Montage_IsPlaying` (`SkeletalMeshComponent.GetAnimInstance` (`self.Mesh`)) (`self.AttackMontage`))))

(fn `is withing attack range?`
  (returns (ReturnValue :type Boolean))
  ; Calculate if the player is within attack range or not.
  (return (< (`self.GetDistanceTo` (`GameplayStatics.GetPlayerCharacter` 0)) (`self.attack range`))))

(fn `Spawn Bullet`
  ; Spawn Bullet at Random Target point after Killing Random Enemy
  (bind _asbp_third_person_game_mode (cast `/Game/DoomEternalGame/Characters/Blueprints/BP_ThirdPersonGameMode` (`GameplayStatics.GetGameMode`)))
  (set `/Game/DoomEternalGame/Characters/Blueprints/BP_ThirdPersonGameMode.Spawn Bullet` (== (`KismetMathLibrary.RandomIntegerInRange` 0 1) 1) _asbp_third_person_game_mode)
  (set `/Game/DoomEternalGame/Characters/Blueprints/BP_ThirdPersonGameMode.Ammo Spawn Point` (`self.spawnPoint`) _asbp_third_person_game_mode))

(fn `UserConstructionScript`)